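; Carjump is a set prop that slides its skeletal mesh back and forth between its origin and HitLocation, using logic labeled as a smasher.
; A timeline scaled by TravelTimeInSeconds drives the lerp, pausing at each end before reversing when the Stopped check passes.
; An attached Vroom sound accompanies movement, with events to halt or resume it.
; The construction script can preview the end position via TestEndLocation.
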(event Custom|SmasherDown
  ;[1 1 1] Smasher Head Engine
  (bind (_direction _lerp_alpha) (Timeline|MoverTimeline PlayFromStart)
    (:Update
      (Variables|Default|SetMoverDirection _direction)
      (CallFunction|MoverHead _lerp_alpha))
    (:Finished
      (Audio|Components|Audio|Stop (stale _moversoundout))
      (Utilities|FlowControl|Delay (Variables|Default|GetStopDelay))
      (if (Variables|Default|GetStopped)
        (switch Utilities|FlowControl|Switch|SwitchonETimelineDirection _direction
          (:Forward
            (CallFunction|SmasherUp)
            (goto _label Reset))
          (:Backward
            (CallFunction|SmasherDown)
            (goto _label Reset)))))
    (:sparksActive
      (Utilities|FlowControl|DoOnce false :!label _label
        (:Completed
          (bind _moversoundout (CallFunction|MoverSound)))))))

(event Custom|StartFromPlay
  ;[1 1 1] Smasher Head Engine
  (Utilities|FlowControl|Sequence
    (:then_0
      (if (Math|Conversions|ToBoolean(Integer) (Math|Conversions|ToInteger(Byte) (Variables|Default|GetMoverDirection)))
        (bind (_direction _lerp_alpha) (Timeline|MoverTimeline Reverse)
          (:Update
            (Variables|Default|SetMoverDirection _direction)
            (CallFunction|MoverHead _lerp_alpha))
          (:Finished
            (Audio|Components|Audio|Stop (stale _moversoundout))
            (Utilities|FlowControl|Delay (Variables|Default|GetStopDelay))
            (if (Variables|Default|GetStopped)
              (switch Utilities|FlowControl|Switch|SwitchonETimelineDirection _direction
                (:Forward
                  (CallFunction|SmasherUp)
                  (goto _label Reset))
                (:Backward
                  (CallFunction|SmasherDown)
                  (goto _label Reset)))))
          (:sparksActive
            (Utilities|FlowControl|DoOnce false :!label _label
              (:Completed
                (bind _moversoundout (CallFunction|MoverSound :!label _label_2))))))
        (else
          (Timeline|MoverTimeline Play))))
    (:then_1
      (goto _label_2))))

(event Custom|SmasherUp
  ;[1 1 1] Smasher Head Engine
  (bind (_direction _lerp_alpha) (Timeline|MoverTimeline ReverseFromEnd)
    (:Update
      (Variables|Default|SetMoverDirection _direction)
      (CallFunction|MoverHead _lerp_alpha))
    (:Finished
      (Audio|Components|Audio|Stop (stale _moversoundout))
      (Utilities|FlowControl|Delay (Variables|Default|GetStopDelay))
      (if (Variables|Default|GetStopped)
        (switch Utilities|FlowControl|Switch|SwitchonETimelineDirection _direction
          (:Forward
            (CallFunction|SmasherUp)
            (goto _label Reset))
          (:Backward
            (CallFunction|SmasherDown)
            (goto _label Reset)))))
    (:sparksActive
      (Utilities|FlowControl|DoOnce false :!label _label
        (:Completed
          (bind _moversoundout (CallFunction|MoverSound)))))))

(event Custom|MoverFullStop
  ;[1 1 1] Smasher Head Engine
  (Audio|Components|Audio|Stop (stale _moversoundout))
  (bind (_direction _lerp_alpha) (Timeline|MoverTimeline Stop)
    (:Update
      (Variables|Default|SetMoverDirection _direction)
      (CallFunction|MoverHead _lerp_alpha))
    (:Finished
      (Audio|Components|Audio|Stop (stale _moversoundout))
      (Utilities|FlowControl|Delay (Variables|Default|GetStopDelay))
      (if (Variables|Default|GetStopped)
        (switch Utilities|FlowControl|Switch|SwitchonETimelineDirection _direction
          (:Forward
            (CallFunction|SmasherUp)
            (goto _label Reset))
          (:Backward
            (CallFunction|SmasherDown)
            (goto _label Reset)))))
    (:sparksActive
      (Utilities|FlowControl|DoOnce false :!label _label
        (:Completed
          (bind _moversoundout (CallFunction|MoverSound)))))))

(event EventBeginPlay
  ;[1 1 1] Set Smasher Speed
  (Components|Timeline|SetPlayRate (Variables|Default|GetMoverTimeline) (/ 5e+01 (Variables|Default|GetTravelTimeInSeconds))))

(fn ConstructionScript
  (Transformation|SetRelativeLocation (Variables|Default|GetSkeletalMesh) (Math|Vector|SelectVector (Variables|LiftControls|GetHitLocation) "0, 0,0.000000" (Variables|Default|GetTestEndLocation)) false false))

(fn MoverSound
  (bind _returnvalue (Audio|SpawnSoundAttached "/Game/SideScrollerBP/Audio/SoundFx/vroom_cue.vroom_cue" (Variables|Default|GetSkeletalMesh) "None" "0, 0, 0" "0, 0, 0" "KeepRelativeOffset" false 1.0 1.0 0.0 "/Game/SetProps/Sounds/DefaultSoundAttenuation.DefaultSoundAttenuation"))
  (return _returnvalue))

(fn MoverHead
  (params (LERPAlpha :type Float%20%28single-precision%29))
  (Variables|Default|SetLERPAlpha LERPAlpha)
  (Transformation|SetRelativeLocation (Variables|Default|GetSkeletalMesh) (Math|Vector|Lerp(Vector) "0, 0,0.000000" (Variables|LiftControls|GetHitLocation) (Variables|Default|GetLERPAlpha)) false false)
  (return))