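; FamilyDeath3 is an actor that stages a death sequence once the game instance's FamilyMembers count drops to zero or below.
; Tick polls that count, and a DoOnce starts a timeline after a short delay.
; The timeline's float track feeds incremental local Z offsets to five skeletal meshes.
; Its event track activates a particle system and plays steam, scream and crowd sounds in 2D.
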(event Custom|ReceiveActorBeginOverlap_Copy
  (params (OtherActor :type Actor%20Object%20Reference)))

(event EventTick
  (params (DeltaSeconds :type Float%20%28single-precision%29))
  (bind _asdl_game_instance (Utilities|Casting|CastToDL_GameInstance (Game|GetGameInstance)))
  (if (<= (Variables|/Game/DeathlessLive/Blueprint/DL_GameInstance.DL_GameInstance_C|GetFamilyMembers _asdl_game_instance) 0)
    (Utilities|FlowControl|DoOnce false
      (:Completed
        (Utilities|FlowControl|Delay 5.0)
        (bind _newtrack_0 (Timeline|Timeline_0 Play)
          (:Update
            (Class|SceneComponent|AddLocalTransform (Variables|Default|GetSkeletalMesh4) (Math|Transform|MakeTransform (Math|Vector|MakeVector 0.0 0.0 _newtrack_0) "0, 0, 0" "2.000000,2.000000,2.000000") false false)
            (Class|SceneComponent|AddLocalTransform (Variables|Default|GetSkeletalMesh) (Math|Transform|MakeTransform (Math|Vector|MakeVector 0.0 0.0 _newtrack_0) "0, 0, 0" "3.000000,3.000000,3.000000") false false))
          (:NewTrack_1
            (Components|Activation|Activate (Variables|Default|GetParticleSystem1) false)
            (Audio|PlaySound2D "/Game/SideScrollerBP/Audio/SoundFx/Crowd/174628__altfuture__steam_Cue.174628__altfuture__steam_Cue")
            (Audio|PlaySound2D "/Game/SideScrollerBP/Audio/SoundFx/Crowd/220623__adriancalzon__scream-05_Cue.220623__adriancalzon__scream-05_Cue")
            (Audio|PlaySound2D "/Game/SideScrollerBP/Audio/SoundFx/Crowd/37234__shades__crowd-ahh-2_Cue.37234__shades__crowd-ahh-2_Cue")))))))

(fn ConstructionScript)