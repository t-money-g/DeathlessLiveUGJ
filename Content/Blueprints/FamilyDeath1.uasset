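; FamilyDeath1 is an actor that stages a family member's death, moving a skeletal mesh and four chains vertically.
; Tick polls the game instance and, once FamilyMembers is two or fewer, plays the Dip timeline once after five seconds.
; A Dip event track toggles the explosion, plays steam, scream and crowd sounds, and sets the shared Bodydunk flag.
; That flag triggers a second one-shot timeline that applies further cumulative Z offsets.
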(event EventActorBeginOverlap
  (params (OtherActor :type Actor%20Object%20Reference)))

(event EventTick
  (params (DeltaSeconds :type Float%20%28single-precision%29))
  (bind _skeletalmesh (Variables|Default|GetSkeletalMesh))
  (bind _chain2 (Variables|Default|Getchain2))
  (bind _asdl_game_instance (Utilities|Casting|CastToDL_GameInstance (Game|GetGameInstance)))
  (if (Variables|/Game/DeathlessLive/Blueprint/DL_GameInstance.DL_GameInstance_C|Getbodydunk _asdl_game_instance)
    (Utilities|FlowControl|DoOnce false
      (:Completed
        (bind _newtrack_0 (Timeline|Timeline_0 Play)
          (:Update
            (Class|SceneComponent|AddLocalTransform _skeletalmesh (Math|Transform|MakeTransform (Math|Vector|MakeVector 0.0 0.0 _newtrack_0) "0, 0, 0" "2.000000,2.000000,2.000000") false false)
            (Class|SceneComponent|AddLocalTransform _chain2 (Math|Transform|MakeTransform (Math|Vector|MakeVector 0.0 0.0 _newtrack_0) "0, 0, 0" "3.000000,3.000000,3.000000") false false)))))
    (elif (<= (Variables|/Game/DeathlessLive/Blueprint/DL_GameInstance.DL_GameInstance_C|GetFamilyMembers _asdl_game_instance) 2)
      (Utilities|FlowControl|DoOnce false
        (:Completed
          (Utilities|FlowControl|Delay 5.0)
          (bind _newtrack_0_2 (Timeline|dip Play)
            (:Update
              (Class|SceneComponent|AddLocalTransform _skeletalmesh (Math|Transform|MakeTransform (Math|Vector|MakeVector 0.0 0.0 _newtrack_0_2) "0, 0, 0" "2.000000,2.000000,2.000000") false false)
              (Class|SceneComponent|AddLocalTransform _chain2 (Math|Transform|MakeTransform (Math|Vector|MakeVector 0.0 0.0 _newtrack_0_2) "0, 0, 0" "3.000000,3.000000,3.000000") false false))
            (:NewTrack_1
              (Components|Activation|ToggleActive (Variables|Default|Getexplosion))
              (Audio|PlaySoundatLocation "/Game/SideScrollerBP/Audio/SoundFx/Crowd/174628__altfuture__steam.174628__altfuture__steam" "0, 0, 0")
              (Audio|PlaySoundatLocation "/Game/SideScrollerBP/Audio/SoundFx/Crowd/239900__thesubber13__scream-1.239900__thesubber13__scream-1" "0, 0, 0")
              (Audio|PlaySoundatLocation "/Game/SideScrollerBP/Audio/SoundFx/Crowd/37234__shades__crowd-ahh-2.37234__shades__crowd-ahh-2" "0, 0, 0")
              (bind _asdl_game_instance_2 (Utilities|Casting|CastToDL_GameInstance (Game|GetGameInstance)))
              (Variables|/Game/DeathlessLive/Blueprint/DL_GameInstance.DL_GameInstance_C|Setbodydunk _asdl_game_instance_2 true))))))))

(fn ConstructionScript)