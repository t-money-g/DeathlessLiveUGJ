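; Room actor that blends the player's view to its own camera on overlap and scrolls it along Y and Z.
; Two box bounds toggle per-axis following on overlap, so Tick snaps RoomCamera to the pawn's coordinate within that bound.
; With neither axis active, VInterpTo eases the camera toward the bound edge the pawn has passed.
; Construction script places camera and bounds from variables; an entrance-box spawning loop is left unconnected.
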(event OnComponentBeginOverlap(ZAxisCameraBound)
  (params (OtherActor :type Actor%20Object%20Reference) (OtherComp :type Primitive%20Component%20Object%20Reference) (OtherBodyIndex :type Integer) (bFromSweep :type Boolean) (SweepResult :type Hit%20Result%20Structure%20%28by%20ref%29))
  (Variables|Default|SetEnableZAxis true))

(event OnComponentBeginOverlap(YaxisCameraBound)
  (params (OtherActor :type Actor%20Object%20Reference) (OtherComp :type Primitive%20Component%20Object%20Reference) (OtherBodyIndex :type Integer) (bFromSweep :type Boolean) (SweepResult :type Hit%20Result%20Structure%20%28by%20ref%29))
  (Variables|Default|SetEnableYaxis true))

(event OnComponentEndOverlap(ZAxisCameraBound)
  (params (OtherActor :type Actor%20Object%20Reference) (OtherComp :type Primitive%20Component%20Object%20Reference) (OtherBodyIndex :type Integer))
  (Variables|Default|SetEnableZAxis false))

(event OnComponentEndOverlap(YaxisCameraBound)
  (params (OtherActor :type Actor%20Object%20Reference) (OtherComp :type Primitive%20Component%20Object%20Reference) (OtherBodyIndex :type Integer))
  (Variables|Default|SetEnableYaxis false))

(event EventBeginPlay
  (Variables|/Script/Engine.CameraComponent|SetFieldOfView (Variables|Default|GetRoomCamera) (Variables|Default|GetFOV)))

(event EventTick
  (params (DeltaSeconds :type Float%20%28single-precision%29))
  (bind _returnvalue (Game|Player|GetPlayerPawn 0))
  (bind _returnvalue_2 (Game|Player|GetPlayerPawn 0))
  (bind _returnvalue_3 (Game|Player|GetPlayerPawn 0))
  (bind _roomcamera (Variables|Default|GetRoomCamera))
  (bind _yaxiscamerabound (Variables|Default|GetYaxisCameraBound))
  (bind _roomcamera_2 (Variables|Default|GetRoomCamera))
  (bind _zaxiscamerabound (Variables|Default|GetZAxisCameraBound))
  (bind _enablezaxis (Variables|Default|GetEnableZAxis))
  (bind _roomcamera_3 (Variables|Default|GetRoomCamera))
  (bind _yaxiscamerabound_2 (Variables|Default|GetYaxisCameraBound))
  (bind _zaxiscamerabound_2 (Variables|Default|GetZAxisCameraBound))
  (bind _returnvalue_4 (Transformation|GetActorLocation _returnvalue))
  (bind _returnvalue_5 (Transformation|GetWorldLocation _roomcamera_2))
  (bind (_origin _boxextent) (Collision|GetComponentBounds _yaxiscamerabound))
  (bind _returnvalue_6 (Transformation|GetWorldLocation _roomcamera))
  (bind (_origin_2 _boxextent_2) (Collision|GetComponentBounds _zaxiscamerabound))
  (bind _returnvalue_7 (Transformation|GetActorLocation _returnvalue_2))
  (bind (_origin_3 _boxextent_3) (Collision|GetComponentBounds _zaxiscamerabound_2))
  (bind _returnvalue_8 (Transformation|GetActorLocation _returnvalue_3))
  (bind _returnvalue_9 (Transformation|GetWorldLocation _roomcamera_3))
  (bind (_origin_4 _boxextent_4) (Collision|GetComponentBounds _yaxiscamerabound_2))
  (bind (_x _y _z) (Math|Vector|BreakVector _returnvalue_5))
  (bind (_x_2 _y_2 _z_2) (Math|Vector|BreakVector _returnvalue_4))
  (bind _returnvalue_10 (- _origin _boxextent))
  (bind _returnvalue_11 (- _origin_2 _boxextent_2))
  (bind _z_3 (Math|Vector|BreakVector _returnvalue_7))
  (bind (_x_3 _y_3 _z_4) (Math|Vector|BreakVector _returnvalue_9))
  (bind _y_4 (Math|Vector|BreakVector _returnvalue_8))
  (bind _returnvalue_12 (+ _origin _boxextent))
  (bind _returnvalue_13 (+ _origin_2 _boxextent_2))
  (Variables|Default|SetDeltaT DeltaSeconds)
  (if (Variables|Default|GetEnableYaxis)
    (if _enablezaxis
      (Utilities|FlowControl|Sequence
        (:then_0
          ;[1 1 1] Y-Axis Camera
          (Transformation|SetWorldLocation _roomcamera_3 (Math|Vector|MakeVector _x_3 (Math|Float|SelectFloat _y_3 _y_4 (or (>= _y_4 (.y (+ _origin_4 _boxextent_4))) (<= _y_4 (.y (- _origin_4 _boxextent_4))))) _z_4) false false :!label _label))
        (:then_1
          ;[1 1 1] Z-Axis Camera
          (Transformation|SetWorldLocation _roomcamera_2 (Math|Vector|MakeVector _x _y (Math|Float|SelectFloat _z _z_3 (or (>= _z_3 (.z (+ _origin_3 _boxextent_3))) (<= _z_3 (.z (- _origin_3 _boxextent_3)))))) false false :!label _label_2)))
      (else
        (goto _label)))
    (elif _enablezaxis
      (goto _label_2)
      (else
        ;[1 1 1] No Camera Axis Active
        (Transformation|SetWorldLocation _roomcamera (Math|Interpolation|VInterpTo (Math|Vector|MakeVector (.x _returnvalue_6) (.y _returnvalue_6) (.z _returnvalue_6)) (Math|Vector|MakeVector (.x _returnvalue_6) (Math|Float|SelectFloat (Math|Float|SelectFloat (.y _returnvalue_12) (.y _returnvalue_10) (>= _y_2 (.Y (Math|Vector|BreakVector _origin)))) (.y _returnvalue_6) (or (>= _y_2 (.y _returnvalue_12)) (<= _y_2 (.y _returnvalue_10)))) (Math|Float|SelectFloat (Math|Float|SelectFloat (.z _returnvalue_13) (.z _returnvalue_11) (>= _z_2 (.Z (Math|Vector|BreakVector _origin_2)))) (.z _returnvalue_6) (or (>= _z_2 (.z _returnvalue_13)) (<= _z_2 (.z _returnvalue_11))))) (Variables|Default|GetDeltaT) 1e+01) false false)))))

(event Collision|EventActorBeginOverlap
  (params (OtherActor :type Actor%20Object%20Reference))
  (Game|Player|SetViewTargetwithBlend (Game|GetPlayerController 0) self (Variables|Default|GetBlendTime) (Variables|Default|GetBlendFunc) (Variables|Default|GetBlendExp) false))

(fn ConstructionScript
  (bind _zaxiscamerabound (Variables|Default|GetZAxisCameraBound))
  (bind _yaxiscamerabound (Variables|Default|GetYaxisCameraBound))
  (Utilities|FlowControl|Sequence
    (:then_1
      (Transformation|SetRelativeTransform (Variables|Default|GetRoomCamera) (Variables|Default|GetCameraTranform) false false))
    (:then_2
      (Transformation|SetRelativeTransform _zaxiscamerabound (Variables|Default|GetZaxisPosistion) false false)
      (Components|Box|SetBoxExtent _zaxiscamerabound (Variables|Default|GetZAxisBoxExtent) true))
    (:then_3
      (Transformation|SetRelativeTransform _yaxiscamerabound (Variables|Default|GetYAxisPosision) false false)
      (Components|Box|SetBoxExtent _yaxiscamerabound (Variables|Default|GetYAxisBoxExtent) true))))