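; Game instance for DeathlessLive that tracks remaining family members, which act as lives, across level loads.
; KillFamMember decrements the count, plays a random voice clip, then disables input, ragdolls the player character and sets it on fire.
; After a delay, if members remain, it opens the map selected by Level and clears StopIntro.
; A separate map1death event only decrements a first-map death counter.
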(event Custom|map1death
  (Variables|Default|SetfamDeathmap1 (- (Variables|Default|GetfamDeathmap1) 1)))

(event Custom|KillFamMember
  (bind _output_get (Variables|Default|SetFamilyMembers (- (Variables|Default|GetFamilyMembers) 1)))
  (Development|PrintString (Utilities|String|ToString(Integer) _output_get))
  (Audio|PlaySound2D (Utilities|Select :Index (Math|Random|RandomIntegerinRange 0 3) :Option%200 "/Game/Voiceover/willnotpachal.willnotpachal" :Option%201 "/Game/Voiceover/allargytofire.allargytofire" :Option%202 "/Game/Voiceover/shellygame.shellygame" :Option%203 "/Game/Voiceover/sosorry.sosorry") 5.0 0.8)
  (bind _ascharacter (Utilities|Casting|CastToCharacter (Game|Player|GetPlayerPawn 0)))
  (Input|DisableInput _ascharacter 0)
  (Physics|SetSimulatePhysics (Variables|/Script/Engine.Character|GetMesh _ascharacter) true)
  (Collision|SetCollisionEnabled (Variables|/Script/Engine.Character|GetMesh _ascharacter) "QueryAndPhysics")
  (Effects|SpawnEmitterAttached "/Game/StarterContent/Particles/P_Fire.P_Fire" (Variables|/Script/Engine.Character|GetMesh _ascharacter) "None")
  (Utilities|FlowControl|Delay 1e+01)
  (if (not (<= (Variables|Default|GetFamilyMembers) 0))
    (Game|OpenLevel(byName) (Utilities|Select :Index (Variables|Default|GetLevel) :Option%200 "DL_Level2" :Option%201 "DL_Level3" :Option%202 "DL_Level4" :Option%203 "DL_Level5"))
    (Variables|Default|SetStopIntro false)))